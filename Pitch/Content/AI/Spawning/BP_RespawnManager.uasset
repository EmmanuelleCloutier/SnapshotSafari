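; BP_RespawnManager respawns herbivore AI at designated respawn points in the level.
; On BeginPlay it collects every BP_RespawnPointHerbivore actor into the RespawnPoint array.
; The RespawningHerbivore event picks a random point from that array, spawns a BP_AIHerbivore at its location and prints a debug message.
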(event Custom|RespawningHerbivore
  (Game|SpawnActorfromClass "/Game/AI/Herbivore/BP_AIHerbivore.BP_AIHerbivore_C" (Math|Conversions|ToTransform(Vector) (Transformation|GetActorLocation (.OutItem (Utilities|Array|Random (Variables|Default|GetRespawnPoint))))) "Undefined" "MultiplyWithRoot" 0 0)
  (Development|PrintString "respawnning herbi"))

(event EventBeginPlay
  (bind _outactors (Actor|GetAllActorsOfClass "/Game/AI/Spawning/BP_RespawnPointHerbivore.BP_RespawnPointHerbivore_C"))
  (for _array_element _outactors
    (Utilities|Array|Add (Variables|Default|GetRespawnPoint) _array_element)))

(fn ConstructionScript)