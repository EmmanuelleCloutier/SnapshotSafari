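; AI controller for a herbivore that switches between behavior trees as danger appears and clears.
; It runs BT_Follow on BeginPlay and on NoMoreDanger, and swaps to BT_FindingCover on SeeDanger.
; The goingtofood event, gated by Complete, writes the indexed FoodLocalisation entry to the Food blackboard key.
; Its length guard compares against -1, so it never catches an empty array.
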(event Custom|going%20to%20food
  ;[1 1 1] Va chercher la nourriture
  (if (Variables|Default|Getcomplete)
    (if (not (== (Utilities|Array|Length (Variables|Default|GetFoodLocalisation)) -1))
      (AI|Components|Blackboard|SetValueasObject (AI|GetBlackboard 0) (Utilities|Name|MakeLiteralName "Food") (Utilities|Array|Get(acopy) (Variables|Default|GetFoodLocalisation) (Variables|Default|Getindexneeded))))))

(event Custom|SeeDanger
  ;[1 1 1] Herbivore finding cover if see danger
  (AI|RunBehaviorTree "/Game/AI/Herbivore/BT_FindingCover.BT_FindingCover"))

(event Custom|NoMoreDanger
  ;[1 1 1] Herbivore finding cover if see danger
  (AI|RunBehaviorTree "/Game/AI/Carnivore/BT_Follow.BT_Follow"))

(event EventBeginPlay
  (AI|RunBehaviorTree "/Game/AI/Carnivore/BT_Follow.BT_Follow"))

(fn ConstructionScript)