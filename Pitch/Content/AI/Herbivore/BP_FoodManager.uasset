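; BP_FoodManager is a trigger actor that creates food for a herbivore AI.
; On BeginPlay it stores a random number of points, up to MaxFood, scattered in X and over the negative-Y half of its box.
; The first BP_AIHerbivore with a BP_HerbivoreController to overlap it triggers a one-time spawn of BP_FoodBase at those points.
; It adds the food to that controller's FoodLocalisation, sets Complete and calls GoingToFood.
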(event Collision|EventActorBeginOverlap
  (params (OtherActor :type Actor%20Object%20Reference))
  ;[1 1 1] Cree la nourriture pour herbivore ou omnivore
  (if (not (Variables|Default|GetAsBeenActivated))
    (bind _asbp_aiherbivore (Utilities|Casting|CastToBP_AIHerbivore OtherActor))
    (Development|PrintString "cast to ai herbi")
    (bind _asbp_herbivore_controller (Utilities|Casting|CastToBP_HerbivoreController (Pawn|GetController _asbp_aiherbivore)))
    (Development|PrintString "cst to controller")
    (Variables|Default|SetAsBeenActivated true)
    (for _array_element (Variables|Default|GetFoodLocalisation)
      (bind _returnvalue (Game|SpawnActorfromClass "/Game/AI/Herbivore/BP_FoodBase.BP_FoodBase_C" (Math|Conversions|ToTransform(Vector) _array_element) "Undefined" "MultiplyWithRoot" 0 0))
      (Development|PrintString "after spawning")
      (Utilities|Array|Add (Variables|/Game/AI/Herbivore/BP_HerbivoreController.BP_HerbivoreController_C|GetFoodLocalisation _asbp_herbivore_controller) _returnvalue))
    (Development|PrintString "finished spawning" true true "(R=0.491982,G=0.284806,B=1.000000,A=1.000000)")
    (Variables|/Game/AI/Herbivore/BP_HerbivoreController.BP_HerbivoreController_C|Setcomplete _asbp_herbivore_controller true)
    (Default|GoingtoFood _asbp_herbivore_controller)))

(event EventBeginPlay
  (bind _returnvalue (Transformation|GetActorLocation))
  (bind _box (Variables|Default|GetBox))
  (bind _returnvalue_2 (Components|Box|GetScaledBoxExtent _box))
  (for _index (range 0 (- (Math|Random|RandomIntegerinRange 1 (Variables|Default|GetMaxFood)) 1))
    (Utilities|Array|Add (Variables|Default|GetFoodLocalisation) (Math|Vector|MakeVector (+ (Math|Random|RandomFloatinRange (* (.x _returnvalue_2) -1.0) (.x _returnvalue_2)) (.x _returnvalue)) (+ (Math|Random|RandomFloatinRange (* (.y _returnvalue_2) -1.0) 0.0) (.y _returnvalue)) (.z _returnvalue_2)))))

(fn ConstructionScript)