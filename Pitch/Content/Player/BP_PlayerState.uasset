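; Player state that holds the player's photo album and current photo index, with persistence through the "SaveSlot" save game.
; BeginPlay restores the index and photos from an existing BP_SaveGame.
; Adding a photo inserts it at the current index, advances the index with wrap-around after 100, then saves.
; Each save creates a fresh save object containing only that new photo and index, replacing the previous save.
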(event Custom|AddPhototoAlbum
  (params (Photo :type Texture%20Render%20Target%202D%20Object%20Reference))
  ;[1 1 1] AjoutePhoto a l'album et enrigistre index ou on est rendu
  (Utilities|Array|Insert (Variables|Default|GetPhotoAlbum) Photo (Variables|Default|GetCurrentIndex))
  (Development|PrintString "photoenrigistrer" true true "(R=1.000000,G=0.986704,B=0.918643,A=1.000000)")
  (CallFunction|AddIndex)
  (CallFunction|EnrigisterPhoto Photo (Variables|Default|GetCurrentIndex)))

(event Custom|AddIndex
  ;[1 1 1] Gerer index de lalbum photo
  (if (== (Variables|Default|GetCurrentIndex) 100)
    (Variables|Default|SetCurrentIndex 0)
    (else
      (Variables|Default|SetCurrentIndex (+ (Variables|Default|GetCurrentIndex) 1)))))

(event Custom|EnrigisterPhoto
  (params (EnrigisterAlbum :type Texture%20Render%20Target%202D%20Object%20Reference) (IndexPhoto :type Integer))
  ;[1 1 1] Gerer enrigistement de partie
  (bind _returnvalue (SaveGame|CreateSaveGameObject "/Game/Player/BP_SaveGame.BP_SaveGame_C"))
  (Variables|/Game/Player/BP_SaveGame.BP_SaveGame_C|SetCurrentIndexPhoto _returnvalue IndexPhoto)
  (Utilities|Array|Add (Variables|/Game/Player/BP_SaveGame.BP_SaveGame_C|GetPhotos _returnvalue) EnrigisterAlbum)
  (bind _returnvalue_2 (SaveGame|SaveGametoSlot _returnvalue "SaveSlot"))
  (Development|PrintString (Utilities|String|ToString(Boolean) _returnvalue_2) true true "(R=0.930123,G=1.000000,B=0.969062,A=1.000000)"))

(event EventBeginPlay
  ;[1 1 1] Upload Save from player
  (bind _returnvalue (SaveGame|DoesSaveGameExist "SaveSlot"))
  (if _returnvalue
    (bind _returnvalue_2 (SaveGame|LoadGamefromSlot "SaveSlot"))
    (bind _asbp_save_game (Utilities|Casting|CastToBP_SaveGame _returnvalue_2))
    ;;[0.4158 0.4269 1] Mettre index from last save
    (Variables|Default|SetCurrentIndex (Variables|/Game/Player/BP_SaveGame.BP_SaveGame_C|GetCurrentIndexPhoto _asbp_save_game))
    ;;[0.3462 0.3532 1] mettre photoalbum from last save
    (for _array_element (Variables|/Game/Player/BP_SaveGame.BP_SaveGame_C|GetPhotos _asbp_save_game)
      (Utilities|Array|Add (Variables|Default|GetPhotoAlbum) _array_element))
    (Development|PrintString "Upload from save complete" true true "(R=0.101929,G=0.220672,B=1.000000,A=1.000000)")))

(fn ConstructionScript)